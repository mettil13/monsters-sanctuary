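; BP_PlayerInteractable is an actor the player clicks to play an interaction animation.
; Clicking calls Interact, which resets its Actor Sequence component's playback position and plays the sequence, so each click restarts it.
; An unused older path that spawned a Level Sequence player for LS_Interaction is left disconnected, noted as not working well.
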(event `self.ReceiveActorOnClicked`
  (params (ButtonPressed :type "Key Structure"))
  (`self.Interact`))

(fn `Interact`
  (bind _actorsequence (`self.ActorSequence`))
  (`MovieSceneSequencePlayer.SetPlaybackPosition` :`self` (`ActorSequenceComponent.SequencePlayer` _actorsequence))
  (`ActorSequenceComponent.PlaySequence` _actorsequence))

(fn `UserConstructionScript`)