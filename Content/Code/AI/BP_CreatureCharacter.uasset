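; Base AI creature character that moves toward a target and owns a CreatureStats component for needs like hunger, thirst and sleep.
; A move event runs AIMoveTo, notifying a finish dispatcher on arrival or printing a red error on failure.
; SetCurrentTarget stores the target, and a debug-style RandomAddStats randomly nudges one need.
; An update loop and stat test calls are left unconnected.
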(event `GoToCurrentGeneralTarget`
  (params (Target :type "Vector Structure"))
  ;[1 1 1] MoveToCurrentTarget
  (`|AIMoveTo` self Target null
    (:`OnSuccess`
      (`KismetSystemLibrary.PrintString` "Target find ( point reached )")
      (`self.OnAIFinishMovingTo`))
    (:`OnFail`
      (`KismetSystemLibrary.PrintString` (`KismetStringLibrary.Concat_StrStr` (`KismetStringLibrary.Concat_StrStr` (`KismetStringLibrary.Concat_StrStr` " the AI " (`KismetSystemLibrary.GetObjectName` self)) " cant reach ") (`KismetSystemLibrary.GetObjectName` (`self.CurrentTarget`))) true true (struct :`R` 1.0 :`B` 0.055084 :`A` 1.0)))))

(event `self.ReceiveBeginPlay`)

(fn `RandomAddStats`
  (bind _messagedurationforrandom (`self.messageDurationForRandom`))
  (bind _creaturestats (`self.CreatureStats`))
  (bind _returnvalue (- (* (`KismetMathLibrary.RandomFloat`) 2.0) 1.0))
  (`KismetSystemLibrary.PrintString` (`KismetStringLibrary.Conv_DoubleToString` _returnvalue))
  (switch `int` (`KismetMathLibrary.RandomInteger` 5)
    (:`0`
      (`/Game/Code/Interfaces/BI_CreatureAI.AddStats` _creaturestats _returnvalue 0.0 0.0 0.0 0.0)
      (`KismetSystemLibrary.PrintString` "added hunger stat" true true (struct :`G` 0.66 :`B` 1.0 :`A` 1.0) _messagedurationforrandom))
    (:`1`
      (`/Game/Code/Interfaces/BI_CreatureAI.AddStats` _creaturestats 0.0 _returnvalue 0.0 0.0 0.0)
      (`KismetSystemLibrary.PrintString` "added thirst stat" true true (struct :`G` 0.66 :`B` 1.0 :`A` 1.0) _messagedurationforrandom))
    (:`2`
      (`/Game/Code/Interfaces/BI_CreatureAI.AddStats` _creaturestats 0.0 0.0 _returnvalue 0.0 0.0)
      (`KismetSystemLibrary.PrintString` "added slumber stat" true true (struct :`G` 0.66 :`B` 1.0 :`A` 1.0) _messagedurationforrandom))
    (:`3`
      (`/Game/Code/Interfaces/BI_CreatureAI.AddStats` _creaturestats 0.0 0.0 0.0 _returnvalue 0.0)
      (`KismetSystemLibrary.PrintString` "added cleanness stat" true true (struct :`G` 0.66 :`B` 1.0 :`A` 1.0) _messagedurationforrandom))
    (:`4`
      (`/Game/Code/Interfaces/BI_CreatureAI.AddStats` _creaturestats 0.0 0.0 0.0 0.0 _returnvalue)
      (`KismetSystemLibrary.PrintString` "added happyness stat" true true (struct :`G` 0.66 :`B` 1.0 :`A` 1.0) _messagedurationforrandom))))

(fn `SetCurrentTarget`
  (params (Target :type "Actor Object Reference"))
  (set `self.CurrentTarget` Target))

(fn `UserConstructionScript`)