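; Generic AI creature character that the player clicks to select, with needs such as hunger, thirst, slumber, cleanness and happiness.
; Clicks toggle selection through the game mode's creatures manager, while select functions swap the overhead widget icon and open or close the HUD stats panel.
; AI MoveTo events broadcast completion on both success and failure, and interactions require the interactable's approval.
; CreatureStats updates every tick, with a debug randomizer for stats.
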(event `GoToNewTarget`
  (params (TargetActor :type "Actor Object Reference"))
  (`|AIMoveTo` self (0.0 0.0 0.0) TargetActor
    (:`OnSuccess`
      _)
    (:`OnFail`
      (`KismetSystemLibrary.PrintString` "Failed" true true (struct :`R` 1.0 :`B` 0.028013 :`A` 1.0))))
  (`self.OnAIFinishMovingTo`))

(event `GoToCurrentGeneralTarget`
  (params (Target :type "Vector Structure"))
  ;[1 1 1] MoveToCurrentTarget
  (`|AIMoveTo` self Target null 40.0
    (:`OnSuccess`
      (`KismetSystemLibrary.PrintString` "Target find ( point reached )"))
    (:`OnFail`
      (`KismetSystemLibrary.PrintString` (`KismetStringLibrary.Concat_StrStr` (`KismetStringLibrary.Concat_StrStr` (`KismetStringLibrary.Concat_StrStr` " the AI " (`KismetSystemLibrary.GetObjectName` self)) " cant reach ") (`KismetStringLibrary.Conv_VectorToString` Target)) true true (struct :`R` 1.0 :`B` 0.055084 :`A` 1.0))))
  (`self.OnAIFinishMovingTo`))

(event `self.ReceiveBeginPlay`
  (`self.UnSelectCreature`))

(event `self.ReceiveTick`
  (params (DeltaSeconds :type "Float (single-precision)"))
  (`/Game/Code/AI/CreatureComponents/BL_Creature.OnTick` (`self.CreatureStats`) DeltaSeconds))

(event `self.ReceiveActorOnClicked`
  (params (ButtonPressed :type "Key Structure"))
  (bind _asbp_camera_game_mode (cast `/Game/Code/GameModes/BP_CameraGameMode` (`GameplayStatics.GetGameMode`)))
  (bind _creaturesmanager (`/Game/Code/GameModes/BP_CameraGameMode.GetCreaturesManager` _asbp_camera_game_mode))
  (if (`self.Selected`)
    (`/Game/Code/GameModeComponents/BP_CreaturesManager.DeselectAll` _creaturesmanager)
    (else
      (`/Game/Code/GameModeComponents/BP_CreaturesManager.SelectCreature` _creaturesmanager self))))

(fn `GetCreatureStats`
  (returns (result :type "CreatureStats Structure"))
  (`KismetSystemLibrary.PrintString` "GettingStats")
  (return (`/Game/Code/AI/CreatureComponents/BL_Creature.stats` (`self.CreatureStats`))))

(fn `InteractWithObjct`
  (params (Interactable :type "/Game/Code/Enviroment/BP_CreatureInteractable Object Reference"))
  (bind _cangiveresource (`/Game/Code/Enviroment/BP_CreatureInteractable.CreatureRequest` Interactable self))
  (if _cangiveresource
    (`/Game/Code/Enviroment/BP_CreatureInteractable.CreatureInteract` Interactable self)
    (else
      (`KismetSystemLibrary.PrintString` "failed to interact"))))

(fn `IsInsideCenter`
  (returns (result :type Boolean))
  (return true))

(fn `RandomAddStats`
  (bind _messagedurationforrandom (`self.messageDurationForRandom`))
  (bind _creaturestats (`self.CreatureStats`))
  (bind _returnvalue (- (* (`KismetMathLibrary.RandomFloat`) 2.0) 1.0))
  (`KismetSystemLibrary.PrintString` (`KismetStringLibrary.Conv_DoubleToString` _returnvalue))
  (switch `int` (`KismetMathLibrary.RandomInteger` 5)
    (:`0`
      (`/Game/Code/Interfaces/BI_CreatureAI.AddStats` _creaturestats _returnvalue 0.0 0.0 0.0 0.0)
      (`KismetSystemLibrary.PrintString` "added hunger stat" true true (struct :`G` 0.66 :`B` 1.0 :`A` 1.0) _messagedurationforrandom))
    (:`1`
      (`/Game/Code/Interfaces/BI_CreatureAI.AddStats` _creaturestats 0.0 _returnvalue 0.0 0.0 0.0)
      (`KismetSystemLibrary.PrintString` "added thirst stat" true true (struct :`G` 0.66 :`B` 1.0 :`A` 1.0) _messagedurationforrandom))
    (:`2`
      (`/Game/Code/Interfaces/BI_CreatureAI.AddStats` _creaturestats 0.0 0.0 _returnvalue 0.0 0.0)
      (`KismetSystemLibrary.PrintString` "added slumber stat" true true (struct :`G` 0.66 :`B` 1.0 :`A` 1.0) _messagedurationforrandom))
    (:`3`
      (`/Game/Code/Interfaces/BI_CreatureAI.AddStats` _creaturestats 0.0 0.0 0.0 _returnvalue 0.0)
      (`KismetSystemLibrary.PrintString` "added cleanness stat" true true (struct :`G` 0.66 :`B` 1.0 :`A` 1.0) _messagedurationforrandom))
    (:`4`
      (`/Game/Code/Interfaces/BI_CreatureAI.AddStats` _creaturestats 0.0 0.0 0.0 0.0 _returnvalue)
      (`KismetSystemLibrary.PrintString` "added happyness stat" true true (struct :`G` 0.66 :`B` 1.0 :`A` 1.0) _messagedurationforrandom))))

(fn `SelectCreature`
  (if (not (`self.Selected`))
    (bind _ascharacter_status (cast `/Game/Code/UI/CharacterStatus` (`WidgetComponent.GetWidget` (`self.WidgetIcon`))))
    (`/Game/Code/UI/CharacterStatus.SetSprite` _ascharacter_status (`self.IconSelected`))
    (set `self.Selected` true)
    (bind _asbp_camera_game_mode (cast `/Game/Code/GameModes/BP_CameraGameMode` (`GameplayStatics.GetGameMode`)))
    (`/Game/Code/UI/WBP_Hud.OpenCreatureStats` (`/Game/Code/GameModes/BP_CameraGameMode.HUD` _asbp_camera_game_mode) self)))

(fn `SetCurrentTarget`
  (params (Target :type "Actor Object Reference"))
  (set `self.CurrentTarget` Target))

(fn `UnSelectCreature`
  (if (`self.Selected`)
    (bind _ascharacter_status (cast `/Game/Code/UI/CharacterStatus` (`WidgetComponent.GetWidget` (`self.WidgetIcon`))))
    (`/Game/Code/UI/CharacterStatus.SetSprite` _ascharacter_status (`self.IconDefault`))
    (set `self.Selected` false)
    (bind _asbp_camera_game_mode (cast `/Game/Code/GameModes/BP_CameraGameMode` (`GameplayStatics.GetGameMode`)))
    (`/Game/Code/UI/WBP_Hud.CloseCreatureStats` (`/Game/Code/GameModes/BP_CameraGameMode.HUD` _asbp_camera_game_mode))))

(fn `UserConstructionScript`)