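; Player camera pawn that pans across a bounded Y/Z plane and focuses on the creature selected in BPCreaturesManager.
; Enhanced Input dragging deselects all creatures and moves the camera using CameraData multipliers and bounds.
; Tick time-lerps toward the selected creature while zooming along X, then zooms back out when selection clears.
; CaptureScene renders a viewport-sized scene capture into a dynamic M_RenderShopItem material, and the pawn registers itself with BP_CameraGameMode.
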(event `self.ReceiveBeginPlay`
  (bind _asplayer_controller (cast `PlayerController` (`self.GetController`)))
  (set `PlayerController.bShowMouseCursor` true _asplayer_controller)
  (set `PlayerController.bEnableClickEvents` true _asplayer_controller)
  (`EnhancedInputSubsystemInterface.AddMappingContext` (pcsubsystem `EnhancedInputLocalPlayerSubsystem` _asplayer_controller) "/Game/Input/IMC_InputMapping.IMC_InputMapping" 0 (struct))
  (bind _asbp_camera_game_mode (cast `/Game/Code/GameModes/BP_CameraGameMode` (`GameplayStatics.GetGameMode`)))
  (set `/Game/Code/GameModes/BP_CameraGameMode.CameraInstance` self _asbp_camera_game_mode))

(event `EnhancedInput|/Game/Input/IA_MoveCamera`
  (params (ActionValue :type Boolean) (ElapsedSeconds :type "Float (double-precision)") (TriggeredSeconds :type "Float (double-precision)") (InputAction :type "InputAction Object Reference" :default "/Game/Input/IA_MoveCamera.IA_MoveCamera"))
  (:`Triggered`
    (set `self.isPanning` ActionValue))
  (:`Completed`
    (set `self.isPanning` false)))

(event `EnhancedInput|/Game/Input/IA_MousePosition`
  (params (ActionValue :type "Vector2D Structure") (ElapsedSeconds :type "Float (double-precision)") (TriggeredSeconds :type "Float (double-precision)") (InputAction :type "InputAction Object Reference" :default "/Game/Input/IA_MousePosition.IA_MousePosition"))
  (:`Triggered`
    (if (`self.isPanning`)
      (bind _asbp_camera_game_mode (cast `/Game/Code/GameModes/BP_CameraGameMode` (`GameplayStatics.GetGameMode`)))
      (`/Game/Code/GameModeComponents/BP_CreaturesManager.DeselectAll` (`/Game/Code/GameModes/BP_CameraGameMode.BP_CreaturesManager` _asbp_camera_game_mode))
      (`self.MoveCameraOffset` ActionValue))))

(event `self.ReceiveTick`
  (params (DeltaSeconds :type "Float (single-precision)"))
  (bind _returnvalue (`KismetMathLibrary.FClamp` (* (- (`self.GetGameTimeSinceCreation`) (`self.StartFocusTime`)) (`/Game/Data/BP_CameraController_DataAsset.FocusLerpSpeed` (`self.CameraData`)))))
  (bind _asbp_camera_game_mode (cast `/Game/Code/GameModes/BP_CameraGameMode` (`GameplayStatics.GetGameMode`)))
  (bind _selectedcreature (`/Game/Code/GameModeComponents/BP_CreaturesManager.SelectedCreature` (`/Game/Code/GameModes/BP_CameraGameMode.BP_CreaturesManager` _asbp_camera_game_mode)))
  (if (== _selectedcreature null)
    (if (`self.IsFocused`)
      (set `self.StartFocusTime` (`self.GetGameTimeSinceCreation`))
      (set `self.IsFocused` false))
    (if (`self.IsFocused`)
      (bind _newposition (`self.LerpZoom` _returnvalue (stale _newposition_3) :!label _label))
      (`self.K2_SetActorLocation` _newposition)
      (else
        (bind _newposition_2 (`self.LerpZoom` (- 1.0 _returnvalue) (`self.K2_GetActorLocation`)))
        (`self.K2_SetActorLocation` _newposition_2)))
    (else
      (if (not (`self.IsFocused`))
        (set `self.StartFocusTime` (`self.GetGameTimeSinceCreation`))
        (set `self.IsFocused` true)
        (set `self.StartFocusLocation` (`self.K2_GetActorLocation`)))
      (bind _newposition_3 (`self.MoveCameraTarget` (`KismetMathLibrary.VLerp` (`self.StartFocusLocation`) (`self.K2_GetActorLocation` _selectedcreature) _returnvalue)))
      (goto _label))))

(fn `CaptureScene`
  (returns (`dynamic material` :type "MaterialInstanceDynamic Object Reference"))
  (bind (_returnvalue_x _returnvalue_y) (`KismetMathLibrary.BreakVector2D` (`WidgetLayoutLibrary.GetViewportSize`)))
  (bind _scenecapturecomponent2d (`self.SceneCaptureComponent2D`))
  (bind _returnvalue (`KismetRenderingLibrary.CreateRenderTarget2D` (`KismetMathLibrary.FTrunc` _returnvalue_x) (`KismetMathLibrary.FTrunc` _returnvalue_y)))
  (bind _output_get (set `SceneCaptureComponent2D.TextureTarget` _returnvalue _scenecapturecomponent2d))
  (`SceneCaptureComponent2D.CaptureScene` _scenecapturecomponent2d)
  (bind _returnvalue_2 (`KismetMaterialLibrary.CreateDynamicMaterialInstance` "/Game/Materials/M_RenderShopItem.M_RenderShopItem"))
  (`MaterialInstanceDynamic.SetTextureParameterValue` _returnvalue_2 "Texture" _output_get)
  (`KismetSystemLibrary.PrintString` "create material dynamic instance")
  (return _returnvalue_2))

(fn `GetSceneCaptureComponent`
  (returns (NewParam :type "SceneCaptureComponent2D Object Reference"))
  (return (`self.SceneCaptureComponent2D`)))

(fn `LerpZoom`
  (params (Alpha :type "Float (double-precision)") (StartPositon :type "Vector Structure"))
  (returns (NewPosition :type "Vector Structure"))
  (bind _cameradata (`self.CameraData`))
  (return (`KismetMathLibrary.MakeVector` (`KismetMathLibrary.Lerp` (.x (`/Game/Data/BP_CameraController_DataAsset.StartPosition` _cameradata)) (`/Game/Data/BP_CameraController_DataAsset.DistanceWhenFocus` _cameradata) Alpha) (.y StartPositon) (.z StartPositon))))

(fn `MoveCameraOffset`
  (params (offset :type "Vector2D Structure"))
  (bind (_x _y) (`KismetMathLibrary.BreakVector2D` offset))
  (bind _cameradata (`self.CameraData`))
  (bind (_x_2 _y_2) (`KismetMathLibrary.BreakVector2D` (`/Game/Data/BP_CameraController_DataAsset.MovementMultiplier` (`self.CameraData`))))
  (`self.K2_SetActorLocation` (`KismetMathLibrary.MakeVector` (.x (`/Game/Data/BP_CameraController_DataAsset.StartPosition` (`self.CameraData`))) (`KismetMathLibrary.FClamp` (.y (+ (* (`KismetMathLibrary.MakeVector` 0.0 (* _x -1.0) (* _y -1.0)) (`KismetMathLibrary.MakeVector` 0.0 _x_2 _y_2)) (`self.K2_GetActorLocation`))) (`/Game/Data/BP_CameraController_DataAsset.LeftBound` _cameradata) (`/Game/Data/BP_CameraController_DataAsset.RightBound` _cameradata)) (`KismetMathLibrary.FClamp` (.z (+ (* (`KismetMathLibrary.MakeVector` 0.0 (* _x -1.0) (* _y -1.0)) (`KismetMathLibrary.MakeVector` 0.0 _x_2 _y_2)) (`self.K2_GetActorLocation`))) (`/Game/Data/BP_CameraController_DataAsset.LowerBound` _cameradata) (`/Game/Data/BP_CameraController_DataAsset.UpperBound` _cameradata)))))

(fn `MoveCameraTarget`
  (params (TargetLocation :type "Vector Structure"))
  (returns (NewPosition :type "Vector Structure"))
  (return (`KismetMathLibrary.MakeVector` (.x (`self.K2_GetActorLocation`)) (.y TargetLocation) (.z TargetLocation))))

(fn `UserConstructionScript`
  (bind _cameradata (`self.CameraData`))
  (`self.K2_SetActorLocation` (`/Game/Data/BP_CameraController_DataAsset.StartPosition` _cameradata))
  (`self.K2_SetActorRotation` (`KismetMathLibrary.Conv_VectorToRotator` (`/Game/Data/BP_CameraController_DataAsset.StartRotation` _cameradata))))