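; BP_CameraGameMode is a game mode that owns the player's money and starts the HUD and shop.
; BeginPlay puts WBP_Hud on screen, initializes the Shop and sets starting Money.
; TryToBuy checks Money against a price and deducts it through AddMoney, returning whether the purchase succeeded.
; AddMoney always calls ClampMoney, which as written zeroes any non-negative balance and leaves negative ones unchanged.
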(event `self.ReceiveBeginPlay`
  (`|ExecutionSequence`
    (:`then_0`
      (bind _returnvalue (`|CreateWidget` "/Game/Code/UI/WBP_Hud.WBP_Hud_C"))
      (`UserWidget.AddToViewport` _returnvalue 0)
      (set `self.HUD` _returnvalue))
    (:`then_1`
      (`Shop.Init` (`self.Shop`)))
    (:`then_2`
      (set `self.Money` 10))))

(fn `AddMoney`
  (params (value :type Integer))
  (set `self.Money` (+ value (`self.Money`)))
  (`self.ClampMoney`))

(fn `ClampMoney`
  (if (<= 0 (`self.Money`))
    (set `self.Money` 0)))

(fn `GetMoney`
  (returns (Money :type Integer))
  (return (`self.Money`)))

(fn `TryToBuy`
  (params (price :type Integer))
  (returns (success :type Boolean))
  (locals (CanBuy :type Boolean))
  (bind _output_get (set `local.CanBuy` (>= (`self.Money`) price)))
  (if _output_get
    (`self.AddMoney` (* price -1)))
  (return _output_get))

(fn `UserConstructionScript`)