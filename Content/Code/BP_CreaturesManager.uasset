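; BP_CreaturesManager keeps the list of creatures and tracks which one is currently selected.
; Creatures are registered and unregistered through simple add and remove functions.
; Selecting a creature unselects every other one in the list, stores the match, then broadcasts a selection-changed event with the stored creature.
; Deselecting all unselects each creature and clears the stored selection without broadcasting that event.
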(fn `AddCreature`
  (params (Creature :type "/Game/Code/AI/BP_CreatureCharacter Object Reference"))
  (`KismetArrayLibrary.Array_Add` (`self.Creatures`) Creature))

(fn `DeselectAll`
  (for _array_element (`self.Creatures`)
    (`/Game/Code/AI/BP_CreatureCharacter.UnSelectCreature` _array_element))
  (set `self.SelectedCreature` null))

(fn `RemoveCreature`
  (params (Creature :type "/Game/Code/AI/BP_CreatureCharacter Object Reference"))
  (returns (Success :type Boolean))
  (bind _returnvalue (`KismetArrayLibrary.Array_RemoveItem` (`self.Creatures`) Creature))
  (return _returnvalue))

(fn `SelectCreature`
  (params (Creature :type "/Game/Code/AI/BP_CreatureCharacter Object Reference"))
  (for _array_element (`self.Creatures`)
    (if (== _array_element Creature)
      (`/Game/Code/AI/BP_CreatureCharacter.SelectCreature` _array_element)
      (set `self.SelectedCreature` _array_element)
      (else
        (`/Game/Code/AI/BP_CreatureCharacter.UnSelectCreature` _array_element))))
  (`self.OnSelectedCreatureChanged` (`self.SelectedCreature`)))