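; BP_InteractableManager is a game mode component that keeps a registry of interactables serving creature needs.
; Add and remove functions sort each interactable by its CreatureNeed into separate arrays for bowls, waters, beds, WCs and toys, covering hunger, thirst, slumber, cleanness and happiness.
; GetAllInteractables rebuilds and returns one combined list from those arrays.
; The event graph holds no logic; the component only acts when its functions are called.
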(fn `Add Interactable`
  (params (Interactable :type "/Game/Code/Enviroment/BP_CreatureInteractable Object Reference"))
  (switch `/Game/Code/AI/Enumerators/E_CreatureNeeds` (`/Game/Code/Enviroment/BP_CreatureInteractable.CreatureNeed` Interactable)
    (:`NewEnumerator0`
      (`KismetArrayLibrary.Array_AddUnique` (`self.Bowls`) Interactable))
    (:`NewEnumerator1`
      (`KismetArrayLibrary.Array_AddUnique` (`self.Waters`) Interactable))
    (:`NewEnumerator2`
      (`KismetArrayLibrary.Array_AddUnique` (`self.Beds`) Interactable))
    (:`NewEnumerator3`
      (`KismetArrayLibrary.Array_AddUnique` (`self.WCs`) Interactable))
    (:`NewEnumerator4`
      (`KismetArrayLibrary.Array_AddUnique` (`self.Toys`) Interactable))))

(fn `GetAllInteractables`
  (returns (Interactables :type "Array of /Game/Code/Enviroment/BP_CreatureInteractable Object Reference"))
  (locals (InteractablesToReturn :type "Array of /Game/Code/Enviroment/BP_CreatureInteractable Object Reference"))
  (bind _interactablestoreturn (`local.InteractablesToReturn`))
  (`KismetArrayLibrary.Array_Clear` _interactablestoreturn)
  (`KismetArrayLibrary.Array_Append` _interactablestoreturn (`self.Bowls`))
  (`KismetArrayLibrary.Array_Append` _interactablestoreturn (`self.Waters`))
  (`KismetArrayLibrary.Array_Append` _interactablestoreturn (`self.Beds`))
  (`KismetArrayLibrary.Array_Append` _interactablestoreturn (`self.WCs`))
  (`KismetArrayLibrary.Array_Append` _interactablestoreturn (`self.Toys`))
  (return _interactablestoreturn))

(fn `RemoveInteractable`
  (params (Interactable :type "/Game/Code/Enviroment/BP_CreatureInteractable Object Reference"))
  (switch `/Game/Code/AI/Enumerators/E_CreatureNeeds` (`/Game/Code/Enviroment/BP_CreatureInteractable.CreatureNeed` Interactable)
    (:`NewEnumerator0`
      (`KismetArrayLibrary.Array_RemoveItem` (`self.Bowls`) Interactable))
    (:`NewEnumerator1`
      (`KismetArrayLibrary.Array_RemoveItem` (`self.Waters`) Interactable))
    (:`NewEnumerator2`
      (`KismetArrayLibrary.Array_RemoveItem` (`self.Beds`) Interactable))
    (:`NewEnumerator3`
      (`KismetArrayLibrary.Array_RemoveItem` (`self.WCs`) Interactable))
    (:`NewEnumerator4`
      (`KismetArrayLibrary.Array_RemoveItem` (`self.Toys`) Interactable))))