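; Game mode component that saves, loads and deletes the player's save slot, which stores the shop's purchased items.
; Saving builds a fresh BP_SaveGameState from the camera game mode's shop, writes it asynchronously, then calls GameSaved on completion.
; SaveGame wraps an event so the async write can run from a function call.
; Loading is synchronous and returns the typed save object without applying it; load and delete first check the slot exists.
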(event `SaveGameEvent`
  (bind _returnvalue (`GameplayStatics.CreateSaveGameObject` "/Game/Code/Saves/BP_SaveGameState.BP_SaveGameState_C"))
  (bind _asbp_camera_game_mode (cast `/Game/Code/GameModes/BP_CameraGameMode` (`GameplayStatics.GetGameMode`))
    (:`then`
      (set `/Game/Code/Saves/BP_SaveGameState.PurchasedItems` (`Shop.PurchasedItems` (`/Game/Code/GameModes/BP_CameraGameMode.Shop` _asbp_camera_game_mode)) _returnvalue))
    (:`CastFailed`
      _))
  (`AsyncActionHandleSaveGame.AsyncSaveGameToSlot` _returnvalue (`self.SaveSlotName`)
    (:`Completed`
      (`self.GameSaved`))))

(fn `DeleteSave`
  (bind _saveslotname (`self.SaveSlotName`))
  (bind _returnvalue (`GameplayStatics.DoesSaveGameExist` _saveslotname))
  (if _returnvalue
    (`GameplayStatics.DeleteGameInSlot` _saveslotname)))

(fn `LoadGame`
  (returns (SaveGameState :type "/Game/Code/Saves/BP_SaveGameState Object Reference"))
  (bind _saveslotname (`self.SaveSlotName`))
  (bind _returnvalue (`GameplayStatics.DoesSaveGameExist` _saveslotname))
  (if _returnvalue
    (bind _returnvalue_2 (`GameplayStatics.LoadGameFromSlot` _saveslotname))
    (bind _asbp_save_game_state (cast `/Game/Code/Saves/BP_SaveGameState` _returnvalue_2))
    (return _asbp_save_game_state)))

(fn `SaveGame`
  (`self.SaveGameEvent`))