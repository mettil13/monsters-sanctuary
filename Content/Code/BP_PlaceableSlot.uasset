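; BP_PlaceableSlot is a slot actor that holds one placeable at its transform, either furniture or a creature interactable, and can swap it on request.
; On BeginPlay it adopts its first attached actor as the current placeable.
; SpawnPlaceable unregisters and destroys the current one, then spawns and attaches the new class.
; Placeables register with the camera game mode's InteractableManager if they are creature interactables, otherwise with its FurnitureManager.
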(event `self.ReceiveBeginPlay`
  (bind _outactors (`self.GetAttachedActors` true))
  (if (> (`KismetArrayLibrary.Array_Length` _outactors) 0)
    (set `self.CurrentPlaceable` (`|GetArrayItem` _outactors))))

(event `PlaceableSlotInterface.SpawnPlaceable`
  (params (placeable :type "Actor Class Reference"))
  (`self.SpawnNewPlaceable` placeable))

(fn `AddCreatureInteractable`
  (params (Interactable :type "/Game/Code/Enviroment/BP_CreatureInteractable Object Reference"))
  (bind _cmaeragamemode (`self.GetCameraGameMode`))
  (bind _interactable_manager (`/Game/Code/GameModes/BP_CameraGameMode.GetInteractableManager` _cmaeragamemode))
  (`/Game/Code/GameModeComponents/BP_InteractableManager.Add Interactable` _interactable_manager Interactable))

(fn `AddFurniture`
  (params (Furniture :type "Actor Object Reference"))
  (bind _cmaeragamemode (`self.GetCameraGameMode`))
  (bind _forniture_manager (`/Game/Code/GameModes/BP_CameraGameMode.GetFurnitureManager` _cmaeragamemode))
  (`KismetArrayLibrary.Array_AddUnique` (`/Game/Code/GameModeComponents/BP_FurnitureManager.furnitures` _forniture_manager) Furniture))

(fn `GetCameraGameMode`
  (returns (CmaeraGameMode :type "/Game/Code/GameModes/BP_CameraGameMode Object Reference"))
  (bind _asbp_camera_game_mode (cast `/Game/Code/GameModes/BP_CameraGameMode` (`GameplayStatics.GetGameMode`))
    (:`then`
      _)
    (:`CastFailed`
      _))
  (return _asbp_camera_game_mode))

(fn `GetId`
  (returns (ReturnValue :type String))
  (return (`self.Id`)))

(fn `RemoveCreatureInteractable`
  (params (Interactable :type "/Game/Code/Enviroment/BP_CreatureInteractable Object Reference"))
  (bind _cmaeragamemode (`self.GetCameraGameMode`))
  (bind _interactable_manager (`/Game/Code/GameModes/BP_CameraGameMode.GetInteractableManager` _cmaeragamemode))
  (`/Game/Code/GameModeComponents/BP_InteractableManager.RemoveInteractable` _interactable_manager Interactable))

(fn `RemoveFurniture`
  (params (Furniture :type "Actor Object Reference"))
  (bind _cmaeragamemode (`self.GetCameraGameMode`))
  (bind _forniture_manager (`/Game/Code/GameModes/BP_CameraGameMode.GetFurnitureManager` _cmaeragamemode))
  (`KismetArrayLibrary.Array_RemoveItem` (`/Game/Code/GameModeComponents/BP_FurnitureManager.furnitures` _forniture_manager) Furniture))

(fn `SpawnNewPlaceable`
  (params (NewPlaceable :type "Actor Class Reference"))
  (bind _currentplaceable (`self.CurrentPlaceable`))
  (bind _currentplaceable_2 (`self.CurrentPlaceable`))
  (if (!= (`self.CurrentPlaceable`) null)
    (bind _asbp_creature_interactable (cast `/Game/Code/Enviroment/BP_CreatureInteractable` _currentplaceable_2)
      (:`then`
        (`self.RemoveCreatureInteractable` _asbp_creature_interactable))
      (:`CastFailed`
        (`self.RemoveFurniture` _currentplaceable_2)))
    (`self.K2_DestroyActor` (`self.CurrentPlaceable`)))
  (bind _returnvalue (`|SpawnActorFromClass` NewPlaceable (`self.GetTransform`) "Undefined" "MultiplyWithRoot" null null))
  (bind _output_get (set `self.CurrentPlaceable` _returnvalue))
  (`self.K2_AttachToActor` _output_get self "None" "SnapToTarget" "SnapToTarget" "SnapToTarget" true)
  (bind _asbp_creature_interactable_2 (cast `/Game/Code/Enviroment/BP_CreatureInteractable` _currentplaceable)
    (:`then`
      (`self.AddCreatureInteractable` _asbp_creature_interactable_2))
    (:`CastFailed`
      (`self.AddFurniture` _currentplaceable))))

(fn `UserConstructionScript`)