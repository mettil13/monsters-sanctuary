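; BP_Interactable is a clickable environment actor that plays an animation sequence when the player clicks it.
; The click event calls PlayerInteract, which sets the playback position of its Actor Sequence component and plays it.
; GetMesh exposes the Cube mesh component.
; An older approach that spawned a Level Sequence player for LS_Interaction remains as unconnected nodes, noted as not working well.
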(event `self.ReceiveActorOnClicked`
  (params (ButtonPressed :type "Key Structure"))
  (`self.PlayerInteract`))

(fn `ffff`)

(fn `GetMesh`
  (returns (Mesh :type "StaticMeshComponent Object Reference"))
  (return (`self.Cube`)))

(fn `PlayerInteract`
  (bind _actorsequence (`self.ActorSequence`))
  (`MovieSceneSequencePlayer.SetPlaybackPosition` :`self` (`ActorSequenceComponent.SequencePlayer` _actorsequence))
  (`ActorSequenceComponent.PlaySequence` _actorsequence))

(fn `UserConstructionScript`)