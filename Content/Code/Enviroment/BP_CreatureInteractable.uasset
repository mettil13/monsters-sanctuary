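; BP_CreatureInteractable is an environment resource that creatures use to raise one need: hunger, thirst, slumber, cleanness or happiness.
; CreatureRequest grants use while Health is above a small threshold, limiting busy objects to CurrentUser, which this graph never assigns.
; CreatureInteract starts a timed InUsing lock, applies the use-related Health change and adds to the matching creature stat.
; Player interaction refills the clamped Health, and Repair resets it directly.
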(event `SetUsing`
  (params (User :type "/Game/Code/AI/BP_CreatureCharacter Object Reference"))
  (set `self.in using` true)
  (`KismetSystemLibrary.Delay` (`self.TimeToWaitBeforeRemoveIsUsing`))
  (set `self.in using` false))

(fn `AddHealth`
  (params (adder :type "Float (double-precision)"))
  (set `self.health` (`KismetMathLibrary.FClamp` (+ adder (`self.health`)))))

(fn `CreatureInteract`
  (params (Crature :type "/Game/Code/AI/BP_CreatureCharacter Object Reference"))
  (bind _creaturestats (`/Game/Code/AI/BP_CreatureCharacter.CreatureStats` Crature))
  (bind _statsadding (`self.statsAdding`))
  (`self.SetUsing` Crature)
  (`self.AddHealth` (`self.healthLossWhenUsed`))
  (switch `/Game/Code/AI/E_CreatureNeeds` (`self.CreatureNeed`)
    (:`NewEnumerator0`
      (`/Game/Code/Interfaces/BI_CreatureAI.AddStats` _creaturestats _statsadding 0.0 0.0 0.0 0.0))
    (:`NewEnumerator1`
      (`/Game/Code/Interfaces/BI_CreatureAI.AddStats` _creaturestats 0.0 _statsadding 0.0 0.0 0.0))
    (:`NewEnumerator2`
      (`/Game/Code/Interfaces/BI_CreatureAI.AddStats` _creaturestats 0.0 0.0 _statsadding 0.0 0.0))
    (:`NewEnumerator3`
      (`/Game/Code/Interfaces/BI_CreatureAI.AddStats` _creaturestats 0.0 0.0 0.0 _statsadding 0.0))
    (:`NewEnumerator4`
      (`/Game/Code/Interfaces/BI_CreatureAI.AddStats` _creaturestats 0.0 0.0 0.0 0.0 _statsadding))))

(fn `CreatureRequest`
  (params (User :type "/Game/Code/AI/BP_CreatureCharacter Object Reference"))
  (returns (canGiveResource :type Boolean))
  (bind _returnvalue (> (`self.health`) 0.1))
  (if (`self.in using`)
    (return (and _returnvalue (== User (`self.CurrentUser`))))
    (else
      (return _returnvalue))))

(fn `PlayerInteract`
  (`KismetSystemLibrary.PrintString` "Player resource repair")
  (`self.AddHealth` 1000.0))

(fn `Repair`
  (set `self.health` 1.0))

(fn `UserConstructionScript`
  (`parent.UserConstructionScript`))