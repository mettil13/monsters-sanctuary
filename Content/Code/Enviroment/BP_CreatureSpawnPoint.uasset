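; Clickable creature spawn point that spawns a monster through its MonsterSpawner and then calls MonsterSpawned.
; Activate asks the camera game mode's creatures manager for spawnable types not yet spawned, and shows the Cube with collision only if any remain.
; Deactivate hides the Cube and disables its collision.
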(event `self.ReceiveActorOnClicked`
  (params (ButtonPressed :type "Key Structure"))
  (`/Game/Code/BP_MonsterSpawner.SpawnMonster` (`self.MonsterSpawner`))
  (`self.MonsterSpawned`))

(fn `Activate`
  (bind _cube (`self.Cube`))
  (bind _asbp_camera_game_mode (cast `/Game/Code/GameModes/BP_CameraGameMode` (`GameplayStatics.GetGameMode`)))
  (bind _creaturesmanager (`/Game/Code/GameModes/BP_CameraGameMode.GetCreaturesManager` _asbp_camera_game_mode))
  (bind _spawnablecreaturestypes (`/Game/Code/GameModeComponents/BP_CreaturesManager.GetSpawnableCreaturesTypesNotAlreadySpawned` _creaturesmanager))
  (if (> (`KismetArrayLibrary.Array_Length` _spawnablecreaturestypes) 0)
    (`SceneComponent.SetVisibility` _cube true false)
    (`PrimitiveComponent.SetCollisionEnabled` _cube "QueryAndPhysics")))

(fn `Deactivate`
  (bind _cube (`self.Cube`))
  (`SceneComponent.SetVisibility` _cube false false)
  (`PrimitiveComponent.SetCollisionEnabled` _cube "NoCollision"))

(fn `GetMesh`
  (returns (Mesh :type "StaticMeshComponent Object Reference"))
  (return (`parent.GetMesh`)))

(fn `UserConstructionScript`
  (`parent.UserConstructionScript`))